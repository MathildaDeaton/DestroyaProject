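; BP_Cars_2 is a car actor that moves along the spline of a referenced RoadTrack when ActiveCar is set at BeginPlay.
; MoveCar scales the CarFollowPath timeline's play rate by Duration, starts it at CarStartOffset and plays it in reverse.
; Each update maps the timeline alpha to a distance along the spline and applies that world location and the unflipped spline rotation to the car.
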(event Custom|MoveCar
  (bind _carfollowpath (Variables|Default|GetCarFollowPath))
  (bind _roadtrack (Variables|Default|GetRoadTrack))
  (bind _roadspline (Variables|/Game/Cars/BP_Tracks.BP_Tracks_C|GetRoadSpline _roadtrack))
  (Components|Timeline|SetPlayRate _carfollowpath (/ 1.0 (Variables|Default|GetDuration)))
  (Components|Timeline|SetNewTime _carfollowpath (Variables|Default|GetCarStartOffset))
  (bind _alpha (Timeline|CarFollowPath Reverse)
    (:Update
      (Variables|Default|SetAlpha _alpha)
      (Transformation|SetActorLocationAndRotation (Spline|GetLocationatDistanceAlongSpline _roadspline (Math|Float|Lerp 0.0 (Spline|GetSplineLength _roadspline) (Variables|Default|GetAlpha)) "World") (Spline|GetRotationatDistanceAlongSpline _roadspline (Math|Float|Lerp 0.0 (Spline|GetSplineLength _roadspline) (Variables|Default|GetAlpha)) "World")))))

(event EventBeginPlay
  (if (Variables|Default|GetActiveCar)
    (CallFunction|MoveCar)))

(fn ConstructionScript)