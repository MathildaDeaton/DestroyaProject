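; BP_WrestleSign is a sign prop whose Plane mesh has its material swapped among three Suplex materials, apparently meant as an animated display.
; BeginPlay starts three looping timers by function name, each aimed at a function that sets one material on the Plane's first slot.
; All timers share the same interval and start together, so the swaps are not staggered.
; No destruction logic is present.
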(event EventBeginPlay
  (Utilities|FlowControl|Sequence
    (:then_0
      (Utilities|Time|SetTimerbyFunctionName 0 "Mat 1" 1.0 true))
    (:then_1
      (Utilities|Time|SetTimerbyFunctionName 0 "Mat 2" 1.0 true))
    (:then_2
      (Utilities|Time|SetTimerbyFunctionName 0 "Mat3" 1.0 true))))

(fn ConstructionScript)

(fn Mat1
  (Rendering|Material|SetMaterial (Variables|Default|GetPlane) 0 "/Game/CustomTextures/Suplex2_Mat.Suplex2_Mat"))

(fn Mat2
  (Rendering|Material|SetMaterial (Variables|Default|GetPlane) 0 "/Game/CustomTextures/Suplex3_Mat.Suplex3_Mat"))

(fn Mat3
  (Rendering|Material|SetMaterial (Variables|Default|GetPlane) 0 "/Game/CustomTextures/Suplex4_Mat.Suplex4_Mat"))