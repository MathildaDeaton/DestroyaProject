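; Master destructible Blueprint that spawns damage debris at hit points for radial and point fractures.
; On authority, two events loop over spawn counts, spawning random classes from DamageChunkMeshes.
; A helper builds each transform using per-axis fixed or random location offsets, with rotation either random or spread around hit direction.
; Both events call the radial spawn-chance check, leaving the point version unused.
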(event EventBeginPlay
  (|CallParentFunction))

(event EventDENTSpawnDamageDebrisPoint
  (params (HitPoint :type Vector :default "0, 0, 0") (HitDirection :type Rotator :default "0, 0, 0"))
  ;[0.2706 0.2706 0.2706] Spawn Damage Debris
  ;;[0.07451 0.1216 0.2706] Get Player Location And Orientation
  ;;;[0.302 0.3647 0.5216] Spawn ProjectilesFrom Point fracture
  (Networking|SwitchHasAuthority
    (:Authority
      (for _index (range 0 (Variables|DENT|DamageChunks|GetSpawnCountPoint))
        (CallFunction|DENTDamageChunksSpawnChanceRadial)
        (bind _returnvalue (CallFunction|DENTDamageChunksSpawnHitpointOffset HitPoint HitDirection))
        ;;;[0.302 0.3647 0.5216] Spawn Random Damage Chunk
        (Game|SpawnActorfromClass (Utilities|RandomValuefromArray (Variables|DENT|DamageChunks|GetDamageChunkMeshes)) _returnvalue "AdjustIfPossibleButAlwaysSpawn" 0 0) ; Spawn projectile
      ))))

(event EventDENTSpawnDamageDebrisRadial
  (params (HitPoint :type Vector :default "0, 0, 0") (HitDirection :type Rotator :default "0, 0, 0"))
  ;[0.2706 0.2706 0.2706] Spawn Damage Debris
  ;;[0.07451 0.1216 0.2706] Get Player Location And Orientation
  ;;;[0.302 0.3647 0.5216] Spawn ProjectilesFrom Radial Fracture
  (Networking|SwitchHasAuthority
    (:Authority
      (for _index (range 0 (- (Variables|DENT|DamageChunks|GetSpawnCountRadial) 1))
        (CallFunction|DENTDamageChunksSpawnChanceRadial)
        (bind _returnvalue (CallFunction|DENTDamageChunksSpawnHitpointOffset HitPoint HitDirection))
        ;;;[0.302 0.3647 0.5216] Spawn Random Damage Chunk
        (Game|SpawnActorfromClass (Utilities|RandomValuefromArray (Variables|DENT|DamageChunks|GetDamageChunkMeshes)) _returnvalue "AdjustIfPossibleButAlwaysSpawn" 0 0) ; Spawn projectile
      ))))

(fn ConstructionScript
  (|CallParentFunction))

(fn DENTDamageChunksSpawnChanceRadial
  ;[0.2706 0.2706 0.2706] Will Chunk Randomly Spawn
  ;;[0.07451 0.1216 0.2706] Bypass Spawn Percentage Check
  (if (Variables|DENT|DamageChunks|GetAlwaysSpawnOnRadial)
    (return)
    (elif (<= (Math|Random|RandomFloatinRange 0.0 1e+02) (Variables|DENT|DamageChunks|GetDamageChunkSpawn%25))
      (return))))

(fn DENTDamageChunksSpawnHitpointOffset
  (params (HitPointIn :type Vector) (HitDirectionIn :type Rotator))
  (bind (_x _y _z) (Math|Vector|BreakVector HitPointIn))
  (bind (_roll _pitch _yaw) (Math|Rotator|BreakRotator HitDirectionIn))
  (bind _spawnrotationoffset (Variables|DENT|DamageChunks|Offset|GetSpawnRotationOffset))
  (bind _spawnspreadoffset (Variables|DENT|DamageChunks|Offset|GetSpawnSpreadOffset))
  (bind (_x_2 _y_2 _z_2) (Math|Vector|BreakVector _spawnspreadoffset))
  (bind (_roll_2 _pitch_2 _yaw_2) (Math|Rotator|BreakRotator _spawnrotationoffset))
  ;[0.2706 0.2706 0.2706] Set Rotation and Location of Spawned Debris
  ;;[0.07451 0.1216 0.2706] Generate Offset location
  ;;;[0.302 0.3647 0.5216] Make Offset For X - Set location or Random location from Offset Spread
  (if (Variables|DENT|DamageChunks|Offset|GetSpawnSpreadLockX)
    (bind _offsetout (Utilities|LockOffSet _x _x_2)
      (:OutPut
        (LocalVariables|SetX _offsetout)))
    (else
      (bind _offsetout_2 (Utilities|SpreadOffSet _x _x_2)
        (:OutPut
          (LocalVariables|SetX _offsetout_2)))))
  ;;;[0.302 0.3647 0.5216] Make Offset For Y - Set location or Random location from Offset Spread
  (if (Variables|DENT|DamageChunks|Offset|GetSpawnSpreadLockY)
    (bind _offsetout_3 (Utilities|LockOffSet _y _y_2)
      (:OutPut
        (LocalVariables|SetY _offsetout_3)))
    (else
      (bind _offsetout_4 (Utilities|SpreadOffSet _y _y_2)
        (:OutPut
          (LocalVariables|SetY _offsetout_4)))))
  ;;;[0.302 0.3647 0.5216] Make Offset For Z - Set location or Random location from Offset Spread
  (if (Variables|DENT|DamageChunks|Offset|GetSpawnSpreadLockZ)
    (bind _offsetout_5 (Utilities|LockOffSet _z _z_2)
      (:OutPut
        (LocalVariables|SetZ _offsetout_5)))
    (else
      (bind _offsetout_6 (Utilities|SpreadOffSet _z _z_2)
        (:OutPut
          (LocalVariables|SetZ _offsetout_6)))))
  ;;[0.07451 0.1216 0.2706] Check if Rotation is random or Set
  (if (Variables|DENT|DamageChunks|Offset|GetRandomRotation)
    ;;[0.07451 0.1216 0.2706] Make Random Rotation Values
    (return (Math|Transform|MakeTransform (Math|Vector|MakeVector (LocalVariables|GetX) (LocalVariables|GetY) (LocalVariables|GetZ)) (Math|Random|RandomRotator false)))
    (else
      (return (Math|Transform|MakeTransform (Math|Vector|MakeVector (LocalVariables|GetX) (LocalVariables|GetY) (LocalVariables|GetZ)) (Math|Rotator|MakeRotator (Math|Random|RandomFloatinRange (+ _roll _roll_2) (- _roll _roll_2)) (Math|Random|RandomFloatinRange (+ _pitch _pitch_2) (- _pitch _pitch_2)) (Math|Random|RandomFloatinRange (+ _yaw _yaw_2) (- _yaw _yaw_2))))))))

(fn DENTDamageChunksSpawnChancePoint
  ;[0.2706 0.2706 0.2706] Will Chunk Randomly Spawn
  ;;[0.07451 0.1216 0.2706] Bypass Spawn Percentage Check
  (if (Variables|DENT|DamageChunks|GetAlwaysSpawnOnPoint)
    (return)
    (elif (<= (Math|Random|RandomFloatinRange 0.0 1e+02) (Variables|DENT|DamageChunks|GetDamageChunkSpawn%25))
      (return))))