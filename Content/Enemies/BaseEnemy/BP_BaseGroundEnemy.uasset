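; Base ground enemy Blueprint with health, a kick reaction, walk/run speeds and projectile firing.
; TakeDamage subtracts a truncated random amount within the given modifiers, while Die separately flags death and hides the health bar.
; KickEnemy launches the physics-simulated mesh along the player's forward vector and upward, polling on a delay until movement is not falling.
; Fire spawns and impulses a projectile, resetting its SpawnProjectile gate immediately.
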(event Custom|Walk
  ;[1 1 1] Movement
  (Variables|/Script/Engine.CharacterMovementComponent|SetMaxWalkSpeed (Variables|Character|GetCharacterMovement) 1.5e+02))

(event Custom|Run
  ;[1 1 1] Movement
  (Variables|/Script/Engine.CharacterMovementComponent|SetMaxWalkSpeed (Variables|Character|GetCharacterMovement) 6e+02))

(event EventTakeDamage
  (params (MinWeaponDamageModifier :type Float%20%28single-precision%29) (MaxWeaponDamageModifier :type Float%20%28single-precision%29) (CritDamageModifier :type Float%20%28single-precision%29) (DamageCauser :type Actor%20Object%20Reference) (HitInfo :type Array%20of%20Hit%20Result%20Structures))
  (bind _output_get (Variables|Default|SetHealth (- (Variables|Default|GetHealth) (Math|Float|Truncate (Math|Random|RandomFloatinRange MinWeaponDamageModifier MaxWeaponDamageModifier))))))

(event EventKickEnemy
  (params (TypeOfKick :type KickMods%20Enum :default "NewEnumerator0"))
  (bind _mesh (Variables|Character|GetMesh))
  ;[1 1 1] Kick
  (Physics|SetSimulatePhysics _mesh true)
  (Physics|AddImpulse _mesh (+ (* (Transformation|GetActorForwardVector (Game|GetPlayerCharacter 0)) 10000) "0, 0,10000.000000") "None" true)
  (Utilities|FlowControl|Delay 5.0 :!label _label)
  (if (AI|Components|NavMovement|IsFalling (Variables|Character|GetCharacterMovement))
    (goto _label)
    (else
      (Physics|SetSimulatePhysics (Variables|Character|GetMesh) false))))

(fn ConstructionScript)

(fn Fire
  (if (Variables|Default|GetSpawnProjectile)
    (bind _returnvalue (Game|SpawnActorfromClass "/Game/FirstPersonBP/Blueprints/FirstPersonProjectile.FirstPersonProjectile_C" (Transformation|GetWorldTransform (Variables|Default|GetSpawnProjectileLocation)) "Undefined" 0 0))
    (Physics|AddImpulse (Variables|/Game/FirstPersonBP/Blueprints/FirstPersonProjectile.FirstPersonProjectile_C|GetSphere _returnvalue) (* (Math|Vector|GetForwardVector (Variables|Character|GetMesh)) (Variables|Default|GetShootForce)) "None" true)
    (Variables|Default|SetSpawnProjectile false)
    (Variables|Default|SetSpawnProjectile true)))

(fn Die
  (params (HitInfo :type Hit%20Result%20Structure))
  (Variables|Default|SetIsDead true)
  (Development|SetHiddeninGame (Variables|Default|GetHealthBar) true false))