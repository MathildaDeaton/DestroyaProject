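; Hackable computer interactable that shows a text prompt when focused and removes itself from the world when interacted with.
; Tick rotates the TextRender each frame to face the player camera, billboard-style.
; Focuson makes the text visible, and no event here hides it again.
; Interact only destroys the actor, with no hacking logic in this Blueprint.
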(event EventInteract
  (Actor|DestroyActor))

(event EventFocuson
  (Rendering|SetVisibility (Variables|Default|GetTextRender) true false))

(event EventTick
  (params (DeltaSeconds :type Float%20%28single-precision%29))
  (bind _textrender (Variables|Default|GetTextRender))
  (Transformation|SetWorldRotation _textrender (Math|Rotator|MakeRotfromX (Math|Vector|NegateVector (- (Transformation|GetWorldLocation _textrender) (Transformation|GetActorLocation (Game|GetPlayerCameraManager 0))))) false false))

(fn ConstructionScript)