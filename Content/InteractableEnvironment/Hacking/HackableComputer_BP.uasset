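; Hackable computer actor that the player hacks by interacting and staying within its overlap area until the required time elapses.
; Focus reveals a text prompt that a looping timer turns toward the camera until the hack completes.
; Interact starts a timer that advances the percentage text, gated on the first-person character's overlap.
; Leaving the area resets progress, hides the text and stops the progress timer.
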(event Custom|Text%20turns%20to%20player
  (bind _textrender (Variables|Default|GetTextRender))
  (Transformation|SetWorldRotation _textrender (Math|Rotator|MakeRotfromX (Math|Vector|NegateVector (- (Transformation|GetWorldLocation _textrender) (Transformation|GetActorLocation (Game|GetPlayerCameraManager 0))))) false false)
  (if (Variables|Default|GetHackCompleted)
    (Utilities|Time|ClearandInvalidateTimerbyHandle (stale EventFocuson _returnvalue))))

(event Custom|UpdateProgress
  (Utilities|FlowControl|Gate true
    (:Exit
      (bind _percentage (CallFunction|GetPercentage (Variables|Default|GetElapsedTime) (Variables|Default|GetRequiredTime)))
      (Variables|Default|SetElapsedTime (+ (Variables|Default|GetTimerUpdateRate) (Variables|Default|GetElapsedTime)))
      (Rendering|Components|TextRender|SetText (Variables|Default|GetTextRender) (Utilities|Text|ToText(String) (Utilities|String|Append (Utilities|String|Append "Hacking " (Utilities|String|ToString(Integer) (Math|Float|Truncate _percentage))) "%")))
      (if (>= _percentage 1e+02)
        (Rendering|Components|TextRender|SetText (Variables|Default|GetTextRender) (Utilities|Text|MakeLiteralText "HACK COMPLETE!"))
        (Variables|Default|SetTimerUpdateRate 0.0)
        (Variables|Default|SetHackCompleted true)
        (Utilities|Time|ClearandInvalidateTimerbyHandle (stale EventInteract _returnvalue))))))

(event EventInteract
  (Utilities|FlowControl|Sequence
    (:then_0
      (Utilities|FlowControl|Gate false) ; enters at Close
    )
    (:then_1
      (bind _returnvalue (Utilities|Time|SetTimerbyEvent (delegate Custom|UpdateProgress) (Variables|Default|GetTimerUpdateRate) true)))))

(event EventFocuson
  (Utilities|FlowControl|Sequence
    (:then_0
      (Utilities|FlowControl|DoOnce false
        (:Completed
          (bind _returnvalue (Utilities|Time|SetTimerbyEvent (delegate Custom|Text%20turns%20to%20player) 0.1 true)))))
    (:then_1
      (Rendering|SetVisibility (Variables|Default|GetTextRender) true false))))

(event EventUnfocus
  (Utilities|FlowControl|Gate false
    (:Exit
      (Rendering|SetVisibility (Variables|Default|GetTextRender) false false))))

(event Collision|EventActorEndOverlap
  (params (OtherActor :type Actor%20Object%20Reference))
  (Utilities|Casting|CastToFirstPersonCharacter OtherActor)
  (Utilities|FlowControl|Sequence
    (:then_0
      (Utilities|FlowControl|Gate true) ; enters at Close
    )
    (:then_1
      (Variables|Default|SetElapsedTime 0.0)
      (Rendering|SetVisibility (Variables|Default|GetTextRender) false false)
      (Rendering|Components|TextRender|SetText (Variables|Default|GetTextRender) (Utilities|Text|MakeLiteralText "Press E to Hack"))
      ;[1 1 1] Replace with Widget/Audio
      (Development|PrintString "Hack Disrupted: Out of Range")
      (Utilities|Time|ClearandInvalidateTimerbyHandle (stale EventInteract _returnvalue)))))

(event Collision|EventActorBeginOverlap
  (params (OtherActor :type Actor%20Object%20Reference))
  (Utilities|Casting|CastToFirstPersonCharacter OtherActor)
  (Utilities|FlowControl|Gate true) ; enters at Open
)

(fn ConstructionScript)

(fn GetPercentage
  (params (LowerValue :type Float%20%28single-precision%29) (MaxValue :type Float%20%28single-precision%29))
  (return (* 100 (/ LowerValue MaxValue))))