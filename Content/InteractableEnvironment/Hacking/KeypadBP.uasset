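; Interactable keypad Blueprint for hacking that checks entered text against a goal code.
; On BeginPlay it hands its WidgetInteraction component to the Keypad widget and binds that widget's Enter press to a check event.
; The check reads text from the KeypadDisplay widget on TargetDisplay, compares it with GoalText, and only prints whether it is correct.
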(event Custom|EnterPreesedEvent
  ;[1 1 1] Comment
  (bind _askeypad_display (Utilities|Casting|CastToKeypadDisplay (UserInterface|GetUserWidgetObject (Variables|/Game/InteractableEnvironment/Hacking/KeypadDisplayBP.KeypadDisplayBP_C|GetWidget (Variables|Default|GetTargetDisplay)))))
  (if (Utilities|Enum|Equal(Enum) (Class|EditableTextBox|GetText (Variables|/Game/InteractableEnvironment/Hacking/KeypadDisplay.KeypadDisplay_C|GetText _askeypad_display)) (Variables|Default|GetGoalText))
    (Development|PrintString "Correct!")
    (else
      (Development|PrintString "Incorrect"))))

(event EventBeginPlay
  ;[1 1 1] Comment
  (bind _askeypad (Utilities|Casting|CastToKeypad (UserInterface|GetUserWidgetObject (Variables|Default|GetWidget))))
  (Variables|/Game/InteractableEnvironment/Hacking/Keypad.Keypad_C|SetWidgetInteraction _askeypad (Variables|Default|GetWidgetInteraction))
  (EventDispatchers|BindEventtoEnterPressed _askeypad (delegate Custom|EnterPreesedEvent)))

(fn ConstructionScript)