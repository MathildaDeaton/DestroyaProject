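; Breakable potted plant prop that falls apart under physics when hit by a FirstPersonProjectile flagged IsProjectile.
; Each mesh part has its own hit event, all calling ALLTHETINGS, which enables physics simulation on the cylinder and five plane meshes.
; Only a hit on the box mesh also releases that mesh and awards destruction points through FirstPersonGameMode, limited to once by a DoOnce.
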(event OnComponentHit(pot_Plane002)
  (params (HitComponent :type Primitive%20Component%20Object%20Reference) (OtherActor :type Actor%20Object%20Reference) (OtherComp :type Primitive%20Component%20Object%20Reference) (NormalImpulse :type Vector :default "0, 0, 0") (Hit :type Hit%20Result%20Structure%20%28by%20ref%29))
  (bind _asfirst_person_projectile (Utilities|Casting|CastToFirstPersonProjectile OtherActor))
  (if (Variables|/Game/FirstPersonBP/Blueprints/FirstPersonProjectile.FirstPersonProjectile_C|GetIsProjectile? _asfirst_person_projectile)
    (CallFunction|ALLTHETINGS)))

(event OnComponentHit(pot_Plane006)
  (params (HitComponent :type Primitive%20Component%20Object%20Reference) (OtherActor :type Actor%20Object%20Reference) (OtherComp :type Primitive%20Component%20Object%20Reference) (NormalImpulse :type Vector :default "0, 0, 0") (Hit :type Hit%20Result%20Structure%20%28by%20ref%29))
  (bind _asfirst_person_projectile (Utilities|Casting|CastToFirstPersonProjectile OtherActor))
  (if (Variables|/Game/FirstPersonBP/Blueprints/FirstPersonProjectile.FirstPersonProjectile_C|GetIsProjectile? _asfirst_person_projectile)
    (CallFunction|ALLTHETINGS)))

(event OnComponentHit(pot_Plane007)
  (params (HitComponent :type Primitive%20Component%20Object%20Reference) (OtherActor :type Actor%20Object%20Reference) (OtherComp :type Primitive%20Component%20Object%20Reference) (NormalImpulse :type Vector :default "0, 0, 0") (Hit :type Hit%20Result%20Structure%20%28by%20ref%29))
  (bind _asfirst_person_projectile (Utilities|Casting|CastToFirstPersonProjectile OtherActor))
  (if (Variables|/Game/FirstPersonBP/Blueprints/FirstPersonProjectile.FirstPersonProjectile_C|GetIsProjectile? _asfirst_person_projectile)
    (CallFunction|ALLTHETINGS)))

(event OnComponentHit(pot_Plane008)
  (params (HitComponent :type Primitive%20Component%20Object%20Reference) (OtherActor :type Actor%20Object%20Reference) (OtherComp :type Primitive%20Component%20Object%20Reference) (NormalImpulse :type Vector :default "0, 0, 0") (Hit :type Hit%20Result%20Structure%20%28by%20ref%29))
  (bind _asfirst_person_projectile (Utilities|Casting|CastToFirstPersonProjectile OtherActor))
  (if (Variables|/Game/FirstPersonBP/Blueprints/FirstPersonProjectile.FirstPersonProjectile_C|GetIsProjectile? _asfirst_person_projectile)
    (CallFunction|ALLTHETINGS)))

(event OnComponentHit(pot_Plane009)
  (params (HitComponent :type Primitive%20Component%20Object%20Reference) (OtherActor :type Actor%20Object%20Reference) (OtherComp :type Primitive%20Component%20Object%20Reference) (NormalImpulse :type Vector :default "0, 0, 0") (Hit :type Hit%20Result%20Structure%20%28by%20ref%29))
  (bind _asfirst_person_projectile (Utilities|Casting|CastToFirstPersonProjectile OtherActor))
  (if (Variables|/Game/FirstPersonBP/Blueprints/FirstPersonProjectile.FirstPersonProjectile_C|GetIsProjectile? _asfirst_person_projectile)
    (CallFunction|ALLTHETINGS)))

(event OnComponentHit(pot_Box001_DM)
  (params (HitComponent :type Primitive%20Component%20Object%20Reference) (OtherActor :type Actor%20Object%20Reference) (OtherComp :type Primitive%20Component%20Object%20Reference) (NormalImpulse :type Vector :default "0, 0, 0") (Hit :type Hit%20Result%20Structure%20%28by%20ref%29))
  (bind _asfirst_person_projectile (Utilities|Casting|CastToFirstPersonProjectile OtherActor))
  (if (Variables|/Game/FirstPersonBP/Blueprints/FirstPersonProjectile.FirstPersonProjectile_C|GetIsProjectile? _asfirst_person_projectile)
    (Physics|SetSimulatePhysics (Variables|Default|Getpot_Box001_DM) true)
    (CallFunction|ALLTHETINGS)
    (Utilities|FlowControl|DoOnce false
      (:Completed
        (bind _asfirst_person_game_mode (Utilities|Casting|CastToFirstPersonGameMode (Game|GetGameMode)))
        (Default|AddDestructionPoints _asfirst_person_game_mode 10)))))

(event OnComponentHit(pot_Cylinder001)
  (params (HitComponent :type Primitive%20Component%20Object%20Reference) (OtherActor :type Actor%20Object%20Reference) (OtherComp :type Primitive%20Component%20Object%20Reference) (NormalImpulse :type Vector :default "0, 0, 0") (Hit :type Hit%20Result%20Structure%20%28by%20ref%29))
  (bind _asfirst_person_projectile (Utilities|Casting|CastToFirstPersonProjectile OtherActor))
  (if (Variables|/Game/FirstPersonBP/Blueprints/FirstPersonProjectile.FirstPersonProjectile_C|GetIsProjectile? _asfirst_person_projectile)
    (CallFunction|ALLTHETINGS)))

(fn ConstructionScript)

(fn ALLTHETINGS
  (Utilities|FlowControl|Sequence
    (:then_0
      (Physics|SetSimulatePhysics (Variables|Default|Getpot_Plane002) true))
    (:then_1
      (Physics|SetSimulatePhysics (Variables|Default|Getpot_Plane006) true))
    (:then_2
      (Physics|SetSimulatePhysics (Variables|Default|Getpot_Plane007) true))
    (:then_3
      (Physics|SetSimulatePhysics (Variables|Default|Getpot_Plane008) true))
    (:then_4
      (Physics|SetSimulatePhysics (Variables|Default|Getpot_Plane009) true))
    (:then_5
      (Physics|SetSimulatePhysics (Variables|Default|Getpot_Cylinder001) true))))