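; BP_MeshToSlice is a sliceable mesh actor that carries a procedural copy of a static mesh.
; The construction script copies MeshToSlice into ProceduralMesh with collision enabled.
; Slicing is not wired up: the event stubs are empty, and disconnected nodes would slice at an overlapping component's location, simulate physics on the new half and print a message.
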(event OnComponentBeginOverlap(ProceduralMesh)
  (params (OverlappedComponent :type Primitive%20Component%20Object%20Reference) (OtherActor :type Actor%20Object%20Reference) (OtherComp :type Primitive%20Component%20Object%20Reference) (OtherBodyIndex :type Integer) (bFromSweep :type Boolean) (SweepResult :type Hit%20Result%20Structure%20%28by%20ref%29))
  ;[1 1 1] DEAD
)

(event EventBeginPlay
  ;[1 1 1] DEAD
)

(event Collision|EventActorBeginOverlap
  (params (OtherActor :type Actor%20Object%20Reference)))

(event EventTick
  (params (DeltaSeconds :type Float%20%28single-precision%29)))

(fn ConstructionScript
  (Class|KismetProceduralMeshLibrary|CopyProceduralMeshfromStaticMeshComponent (Variables|Default|GetMeshToSlice) 0 (Variables|Default|GetProceduralMesh) true))