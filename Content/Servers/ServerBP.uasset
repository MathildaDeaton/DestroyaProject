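; Destructible server actor with four server components, meant to award destruction points and explode at the actor's location when a server's health runs out.
; A Delay loop in BeginPlay re-sums the four health values into ServerHealth; the total-destroyed check only repeats while that sum is depleted.
; Projectile hits write the reduced value to ServerHealth instead of the component's own health, so the per-server DoOnce destruction branches never fire.
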(event OnComponentHit(Server1)
  (params (HitComponent :type Primitive%20Component%20Object%20Reference) (OtherActor :type Actor%20Object%20Reference) (OtherComp :type Primitive%20Component%20Object%20Reference) (NormalImpulse :type Vector :default "0, 0, 0") (Hit :type Hit%20Result%20Structure%20%28by%20ref%29))
  (Utilities|Casting|CastToFirstPersonProjectile OtherActor)
  (Variables|Default|SetServerHealth (- (Variables|Default|GetServer1Health) 2.0))
  (if (<= (Variables|Default|GetServer1Health) 0.0)
    (Utilities|FlowControl|Sequence
      (:then_0
        (Utilities|FlowControl|DoOnce false
          (:Completed
            (bind _asfirst_person_game_mode (Utilities|Casting|CastToFirstPersonGameMode (Game|GetGameMode)))
            (Default|AddDestructionPoints _asfirst_person_game_mode 300)
            (CallFunction|HandleBehavior))))
      (:then_1
        (Development|PrintString "ServerDestroyed")))))

(event OnComponentHit(Server2)
  (params (HitComponent :type Primitive%20Component%20Object%20Reference) (OtherActor :type Actor%20Object%20Reference) (OtherComp :type Primitive%20Component%20Object%20Reference) (NormalImpulse :type Vector :default "0, 0, 0") (Hit :type Hit%20Result%20Structure%20%28by%20ref%29))
  (Utilities|Casting|CastToFirstPersonProjectile OtherActor)
  (Variables|Default|SetServerHealth (- (Variables|Default|GetServer2Health) 2.0))
  (if (<= (Variables|Default|GetServer2Health) 0.0)
    (Utilities|FlowControl|Sequence
      (:then_0
        (Utilities|FlowControl|DoOnce false
          (:Completed
            (bind _asfirst_person_game_mode (Utilities|Casting|CastToFirstPersonGameMode (Game|GetGameMode)))
            (Default|AddDestructionPoints _asfirst_person_game_mode 300)
            (CallFunction|HandleBehavior))))
      (:then_1
        (Development|PrintString "ServerDestroyed")))))

(event OnComponentHit(Server3)
  (params (HitComponent :type Primitive%20Component%20Object%20Reference) (OtherActor :type Actor%20Object%20Reference) (OtherComp :type Primitive%20Component%20Object%20Reference) (NormalImpulse :type Vector :default "0, 0, 0") (Hit :type Hit%20Result%20Structure%20%28by%20ref%29))
  (Utilities|Casting|CastToFirstPersonProjectile OtherActor)
  (Variables|Default|SetServerHealth (- (Variables|Default|GetServer3Health) 2.0))
  (if (<= (Variables|Default|GetServer3Health) 0.0)
    (Utilities|FlowControl|Sequence
      (:then_0
        (Utilities|FlowControl|DoOnce false
          (:Completed
            (bind _asfirst_person_game_mode (Utilities|Casting|CastToFirstPersonGameMode (Game|GetGameMode)))
            (Default|AddDestructionPoints _asfirst_person_game_mode 300)
            (CallFunction|HandleBehavior))))
      (:then_1
        (Development|PrintString "ServerDestroyed")))))

(event OnComponentHit(Server4)
  (params (HitComponent :type Primitive%20Component%20Object%20Reference) (OtherActor :type Actor%20Object%20Reference) (OtherComp :type Primitive%20Component%20Object%20Reference) (NormalImpulse :type Vector :default "0, 0, 0") (Hit :type Hit%20Result%20Structure%20%28by%20ref%29))
  (Utilities|Casting|CastToFirstPersonProjectile OtherActor)
  (Variables|Default|SetServerHealth (- (Variables|Default|GetServer4Health) 2.0))
  (if (<= (Variables|Default|GetServer4Health) 0.0)
    (Utilities|FlowControl|Sequence
      (:then_0
        (Utilities|FlowControl|DoOnce false
          (:Completed
            (bind _asfirst_person_game_mode (Utilities|Casting|CastToFirstPersonGameMode (Game|GetGameMode)))
            (Default|AddDestructionPoints _asfirst_person_game_mode 300)
            (CallFunction|HandleBehavior))))
      (:then_1
        (Development|PrintString "ServerDestroyed")))))

(event EventBeginPlay
  (Utilities|FlowControl|Sequence
    (:then_0
      (Variables|Default|SetServer1Health 1e+02))
    (:then_1
      (Variables|Default|SetServer2Health 1e+02))
    (:then_2
      (Variables|Default|SetServer3Health 1e+02))
    (:then_3
      (Variables|Default|SetServer4Health 1e+02))
    (:then_4
      (Variables|Default|SetServerHealth (+ (Variables|Default|GetServer1Health) (Variables|Default|GetServer2Health) (Variables|Default|GetServer3Health) (Variables|Default|GetServer4Health)) :!label _label)
      (Utilities|FlowControl|Delay 0.1)
      (goto _label))
    (:then_5
      (if (<= (Variables|Default|GetServerHealth) 0.0) :!label _label_2
        (Default|CallServerDestroyed)
        (Utilities|FlowControl|Delay 0.1)
        (goto _label_2)))))

(fn ConstructionScript
  (Variables|Default|SetServerHealth 1e+02))

(fn HandleBehavior
  (Effects|SpawnEmitteratLocation "/Game/StarterContent/Particles/P_Explosion.P_Explosion" (Transformation|GetActorLocation) "0, 0, 0" "2.000000,2.000000,2.000000"))