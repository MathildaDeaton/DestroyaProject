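; BP_BaseWeapon is a base weapon Blueprint that tracks magazine and inventory ammo.
; BeginPlay fills both counts to their maximums, and Fire only decrements the magazine, with no empty check.
; Reload sets the magazine to the lesser of its capacity or the inventory and subtracts that amount, discarding rounds still loaded.
; Query functions report whether the magazine has ammo or is full and whether inventory ammo remains.
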(event EventBeginPlay
  (Variables|Default|SetCurrentAmmoInMag (Variables|Default|GetMaxAmmoInMag))
  (Variables|Default|SetCurrentAmmoInInventory (Variables|Default|GetMaxAmmoInInventory)))

(event Collision|EventActorBeginOverlap
  (params (OtherActor :type Actor%20Object%20Reference)))

(event EventTick
  (params (DeltaSeconds :type Float%20%28single-precision%29)))

(fn ConstructionScript)

(fn Fire
  (Math|Integer|DecrementInt (Variables|Default|GetCurrentAmmoInMag)))

(fn Reload
  (Variables|Default|SetCurrentAmmoInMag (Math|Integer|Min(Integer) (Variables|Default|GetMaxAmmoInMag) (Variables|Default|GetCurrentAmmoInInventory)))
  (Variables|Default|SetCurrentAmmoInInventory (- (Variables|Default|GetCurrentAmmoInInventory) (Math|Integer|Min(Integer) (Variables|Default|GetMaxAmmoInMag) (Variables|Default|GetCurrentAmmoInInventory)))))

(fn HaveAmmoinMag
  (bind _currentammoinmag (Variables|Default|GetCurrentAmmoInMag))
  (return (> _currentammoinmag 0) (== _currentammoinmag (Variables|Default|GetMaxAmmoInMag))))

(fn HaveAmmoinInventory
  (return (> (Variables|Default|GetCurrentAmmoInInventory) 0)))